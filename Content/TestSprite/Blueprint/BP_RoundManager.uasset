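; BP_RoundManager manages round flow for a two-fighter match.
; It saves both fighters' health and locations, then resets each to its saved location, restoring health through the fighter's own ResetHealth rather than the saved value.
; StartRound plays one of three cues based on the zero-based round number it receives, and IncreaseRound advances the round counter.
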(event Custom|ResetFighters
  (params (Player1 :type Player%20Test%20Object%20Reference) (Player2 :type Player%20Test%20Object%20Reference))
  (Default|ResetHealth Player1)
  (Default|ResetLocation Player1 (Variables|Default|GetPlayer1Location))
  (Default|ResetHealth Player2)
  (Default|ResetLocation Player2 (Variables|Default|GetPlayer2Location)))

(event Custom|StartRound
  (params (RoundNumber :type Integer))
  (switch int RoundNumber
    (:0
      (Audio|Components|Audio|Play (Variables|Default|GetRound1Cue) 0.0))
    (:1
      (Audio|Components|Audio|Play (Variables|Default|GetRound2Cue) 0.0))
    (:2
      (Audio|Components|Audio|Play (Variables|Default|GetRound3Cue) 0.0))))

(event Custom|IncreaseRound
  (Math|Integer|IncrementInt (Variables|Default|GetRoundNumber)))

(event Custom|StoreFighters
  (params (Player1 :type Player%20Test%20Object%20Reference) (Player2 :type Player%20Test%20Object%20Reference))
  (Variables|Default|SetPlayer1Health (Variables|/Game/TestSprite/Blueprint/Player_test.Player_test_C|GetHealth Player1))
  (Variables|Default|SetPlayer1Location (Transformation|GetActorLocation Player1))
  (Variables|Default|SetPlayer2Health (Variables|/Game/TestSprite/Blueprint/Player_test.Player_test_C|GetHealth Player2))
  (Variables|Default|SetPlayer2Location (Transformation|GetActorLocation Player2)))

(fn ConstructionScript)