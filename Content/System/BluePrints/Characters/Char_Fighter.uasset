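; Fighter character Blueprint that handles left and right movement for two local players.
; A custom init event adds the IAC_Fighter mapping context to its player controller's Enhanced Input subsystem.
; Separate p1 and p2 input actions push movement along world X on player pawns 0 and 1 by index, rather than on the character itself.
; A node disabling Box collision is left unconnected.
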(event Custom|Init_LocalSubSys
  (bind _asplayer_controller (Utilities|Casting|CastToPlayerController (Pawn|GetController)))
  (Input|AddMappingContext (PlayerController|LocalPlayerSubsystems|GetEnhancedInputLocalPlayerSubsystem _asplayer_controller) "/Game/System/Input/Contexts/IAC_Fighter.IAC_Fighter" 0 "(bIgnoreAllPressedKeysUntilRelease=True,bForceImmediately=False,bNotifyUserSettings=False)"))

(event Input|EnhancedActionEvents|EnhancedInputActionIA_p1Left
  (params (ActionValue :type Boolean) (ElapsedSeconds :type Float%20%28double-precision%29) (TriggeredSeconds :type Float%20%28double-precision%29) (InputAction :type Input%20Action%20Object%20Reference :default "/Game/System/Input/Actions/Input/Inputs_p1/IA_p1Left.IA_p1Left"))
  (Pawn|Input|AddMovementInput (Game|Player|GetPlayerPawn 0) "-1.000000,0.000000,0.000000" 1.0 false))

(event Input|EnhancedActionEvents|EnhancedInputActionIA_p2Left
  (params (ActionValue :type Boolean) (ElapsedSeconds :type Float%20%28double-precision%29) (TriggeredSeconds :type Float%20%28double-precision%29) (InputAction :type Input%20Action%20Object%20Reference :default "/Game/System/Input/Actions/Input/Inputs_p2/IA_p2Left.IA_p2Left"))
  (Pawn|Input|AddMovementInput (Game|Player|GetPlayerPawn 1) "-1.000000,0.000000,0.000000" 1.0 false))

(event Input|EnhancedActionEvents|EnhancedInputActionIA_p1Right
  (params (ActionValue :type Boolean) (ElapsedSeconds :type Float%20%28double-precision%29) (TriggeredSeconds :type Float%20%28double-precision%29) (InputAction :type Input%20Action%20Object%20Reference :default "/Game/System/Input/Actions/Input/Inputs_p1/IA_p1Right.IA_p1Right"))
  (Pawn|Input|AddMovementInput (Game|Player|GetPlayerPawn 0) "1.000000,0.000000,0.000000" 1.0 false))

(event Input|EnhancedActionEvents|EnhancedInputActionIA_p2Right
  (params (ActionValue :type Boolean) (ElapsedSeconds :type Float%20%28double-precision%29) (TriggeredSeconds :type Float%20%28double-precision%29) (InputAction :type Input%20Action%20Object%20Reference :default "/Game/System/Input/Actions/Input/Inputs_p2/IA_p2Right.IA_p2Right"))
  (Pawn|Input|AddMovementInput (Game|Player|GetPlayerPawn 1) "1.000000,0.000000,0.000000" 1.0 false))

(fn ConstructionScript)